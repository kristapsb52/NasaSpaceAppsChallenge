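; Player Blueprint that provides touch-drag camera look, zeroes the player character's gravity and sets up the on-screen UI.
; Touch press stores a start point; each tick, drags beyond a small dead zone add fixed-step yaw or pitch along the dominant axis while held.
; Release clears the pressed flag, then re-enters that drag logic, which only updates the end point.
; BeginPlay adds three widgets to the viewport, with InGame_Interface_Widget initially hidden.
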(event `self.ReceiveTick`
  (params (DeltaSeconds :type "Float (single-precision)"))
  (bind (_locationx _locationy) (`PlayerController.GetInputTouchState` (`GameplayStatics.GetPlayerController` 0) "Touch1"))
  (bind _returnvalue (`KismetMathLibrary.MakeVector2D` _locationx _locationy))
  (bind (_x _y) (`KismetMathLibrary.BreakVector2D` (- (`self.Touch Start 2D Vector`) (`self.Touch End 2D Vector`))))
  (`|ExecutionSequence`
    (:`then_0`
      (if true
        (if (> (`KismetMathLibrary.VSize2D` (- (`self.Touch Start 2D Vector`) _returnvalue)) 10.0)
          (set `self.Touch End 2D Vector` _returnvalue :!label _label)
          (if (`self.isPressed`)
            (if (> (`KismetMathLibrary.Abs` _x) (`KismetMathLibrary.Abs` _y))
              (if (> _x 0.0)
                (`self.AddControllerYawInput` 1.0)
                (else
                  (`self.AddControllerYawInput` -1.0)))
              (elif (> _y 0.0)
                (`self.AddControllerPitchInput` 1.0)
                (else
                  (`self.AddControllerPitchInput` -1.0))))))))))

(event `InputAction|Touch`
  (params (Key :type "Key Structure"))
  (bind (_locationx _locationy) (`PlayerController.GetInputTouchState` (`GameplayStatics.GetPlayerController` 0) "Touch1"))
  (:`Pressed`
    (set `self.isPressed` true)
    (set `self.Touch Start 2D Vector` (`KismetMathLibrary.MakeVector2D` _locationx _locationy)))
  (:`Released`
    (set `self.isPressed` false)
    (goto _label)))

(event `self.ReceiveBeginPlay`
  (set `CharacterMovementComponent.GravityScale` 0.0 (`Character.CharacterMovement` (`GameplayStatics.GetPlayerCharacter` 0)))
  (bind _returnvalue (`|CreateWidget` "/Game/Blueprints/Widgets/In-Game_Interface_Widget1.In-Game_Interface_Widget1_C"))
  (bind _output_get (set `self.NewVar_2` _returnvalue))
  (`UserWidget.AddToViewport` _output_get 0)
  (`Widget.SetVisibility` _output_get "Visible")
  (bind _returnvalue_2 (`|CreateWidget` "/Game/Blueprints/Widgets/UserInterface_Widget.UserInterface_Widget_C"))
  (bind _output_get_2 (set `self.NewVar_1` _returnvalue_2))
  (`UserWidget.AddToViewport` _output_get_2 0)
  (`Widget.SetVisibility` _output_get_2 "Visible")
  (bind _returnvalue_3 (`|CreateWidget` "/Game/Blueprints/Widgets/In-Game_Interface_Widget.In-Game_Interface_Widget_C"))
  (bind _output_get_3 (set `self.NewVar_3` _returnvalue_3))
  (`UserWidget.AddToViewport` _output_get_3 0)
  (`Widget.SetVisibility` _output_get_3 "Hidden"))

(fn `UserConstructionScript`)