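; Point-of-interest actor Blueprint for NGTS-1b that opens an info panel when touched.
; A touch on its Plane component creates an ObjectInfo_NGTS1b widget for the first player, adds it to the viewport and makes it visible.
; Each touch creates a fresh widget with no check for an existing one; the construction script adds nothing beyond the parent call.
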(event `self.Plane.OnInputTouchBegin`
  (params (FingerIndex :type "ETouchIndex Enum" :default "Touch1") (TouchedComponent :type "PrimitiveComponent Object Reference"))
  (bind _returnvalue (`|CreateWidget` "/Game/Blueprints/Widgets/PointsOfInterest/ObjectInfo_NGTS-1b.ObjectInfo_NGTS-1b_C" (`GameplayStatics.GetPlayerController` 0)))
  (bind _output_get (set `self.NewVar_0` _returnvalue))
  (`UserWidget.AddToViewport` _output_get 0)
  (`Widget.SetVisibility` _output_get "Visible"))

(fn `UserConstructionScript`
  (`parent.UserConstructionScript`))