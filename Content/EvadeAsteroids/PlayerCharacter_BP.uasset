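; Player character for the Evade Asteroids game, dodging sideways along Y through touch drags, with gravity disabled at BeginPlay.
; Tick compares the current touch point to the press point and, for held, mostly horizontal drags, nudges the Mesh component a fixed step per frame within bounds.
; Only the mesh is moved, without sweep.
; A capsule hit pauses the game and shows the Game Over widget.
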(event `self.ReceiveTick`
  (params (DeltaSeconds :type "Float (single-precision)"))
  (bind _returnvalue (`GameplayStatics.GetPlayerCharacter` 0))
  (bind _mesh (`self.Mesh`))
  (bind (_locationx _locationy) (`PlayerController.GetInputTouchState` (`GameplayStatics.GetPlayerController` 0) "Touch1"))
  (bind _returnvalue_2 (`KismetMathLibrary.MakeVector2D` _locationx _locationy))
  (bind (_returnvalue_x _returnvalue_y _returnvalue_z) (`KismetMathLibrary.BreakVector` (`SceneComponent.K2_GetComponentLocation` (`Character.Mesh` _returnvalue))))
  (bind (_x _y) (`KismetMathLibrary.BreakVector2D` (- (`self.Touch Start 2D Vector`) (`self.Touch End 2D Vector`))))
  (bind (_returnvalue_x_2 _returnvalue_y_2) (`KismetMathLibrary.BreakVector` (`SceneComponent.K2_GetComponentLocation` (`Character.Mesh` _returnvalue))))
  (`|ExecutionSequence`
    (:`then_0`
      (if true
        (if (> (`KismetMathLibrary.VSize2D` (- (`self.Touch Start 2D Vector`) _returnvalue_2)) 10.0)
          (set `self.Touch End 2D Vector` _returnvalue_2 :!label _label)
          (if (`self.isPressed`)
            (if (> (`KismetMathLibrary.Abs` _x) (`KismetMathLibrary.Abs` _y))
              (if (> _x 0.0)
                (if (not (>= _returnvalue_y_2 (`self.BoundsMax`)))
                  (`SceneComponent.K2_SetWorldLocation` _mesh (`KismetMathLibrary.MakeVector` _returnvalue_x (+ _returnvalue_y 1.0) _returnvalue_z) false false))
                (elif (not (<= _returnvalue_y_2 (`self.BoundsMin`)))
                  (`SceneComponent.K2_SetWorldLocation` _mesh (`KismetMathLibrary.MakeVector` _returnvalue_x (+ _returnvalue_y -1.0) _returnvalue_z) false false))))))))))

(event `InputAction|Touch`
  (params (Key :type "Key Structure"))
  (bind (_locationx _locationy) (`PlayerController.GetInputTouchState` (`GameplayStatics.GetPlayerController` 0) "Touch1"))
  (:`Pressed`
    (set `self.isPressed` true)
    (set `self.Touch Start 2D Vector` (`KismetMathLibrary.MakeVector2D` _locationx _locationy)))
  (:`Released`
    (set `self.isPressed` false)
    (goto _label)))

(event `self.ReceiveBeginPlay`
  (set `CharacterMovementComponent.GravityScale` 0.0 (`Character.CharacterMovement` (`GameplayStatics.GetPlayerCharacter` 0))))

(event `self.CapsuleComponent.OnComponentHit`
  (params (HitComponent :type "PrimitiveComponent Object Reference") (OtherActor :type "Actor Object Reference") (OtherComp :type "PrimitiveComponent Object Reference") (NormalImpulse :type "Vector Structure") (Hit :type "HitResult Structure (by ref)"))
  (`GameplayStatics.SetGamePaused` true)
  (bind _returnvalue (`|CreateWidget` "/Game/Blueprints/Widgets/GameOver_Widget.GameOver_Widget_C"))
  (bind _output_get (set `self.NewVar_0` _returnvalue))
  (`UserWidget.AddToViewport` _output_get 0)
  (`Widget.SetVisibility` _output_get "Visible"))

(fn `UserConstructionScript`)